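; BPC_AudioManager is an actor component that plays random monologue sounds attached to its owner's root component.
; On BeginPlay it spawns a random pick from the Monologue array, then immediately fires its MonologueEnd dispatcher without waiting for playback to finish.
; That event starts a one-minute looping timer whose callback invalidates the handle and plays another monologue, repeating the cycle.
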(event Custom|OnMonologueEnd
  (bind _returnvalue (Utilities|Time|SetTimerbyEvent (delegate Custom|PlayNewMonologue) 6e+01 true)))

(event Custom|PlayNewMonologue
  (Utilities|Time|InvalidateTimerHandle (stale Custom|OnMonologueEnd _returnvalue))
  (bind _newparam (CallFunction|GetRandomMonologue))
  (Audio|SpawnSoundAttached _newparam (Variables|/Script/Engine.Actor|GetRootComponent (Components|GetOwner)) "None" "0, 0, 0" "0, 0, 0" "KeepRelativeOffset" false 1.0 1.0 0.0 0 0)
  (Default|CallMonologueEnd))

(event EventBeginPlay
  (EventDispatchers|BindEventtoMonologueEnd (delegate Custom|OnMonologueEnd))
  (bind _newparam (CallFunction|GetRandomMonologue))
  (Audio|SpawnSoundAttached _newparam (Variables|/Script/Engine.Actor|GetRootComponent (Components|GetOwner)) "None" "0, 0, 0" "0, 0, 0" "KeepRelativeOffset" false 1.0 1.0 0.0 0 0)
  (Default|CallMonologueEnd))

(event EventTick
  (params (DeltaSeconds :type Float%20%28single-precision%29)))

(fn GetRandomMonologue
  (return (.OutItem (Utilities|Array|Random (Variables|Default|GetMonologue)))))