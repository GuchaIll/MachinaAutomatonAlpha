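; BP_MPlayerController is a player controller that tracks current and previous characters for switching possession.
; BeginPlay caches the player's MCharacter as CurrentCharacter.
; SwitchToNextCharacter shifts the current character to PrevCharacter, stores the new one, then possesses PrevCharacter, the outgoing character, rather than the new one.
; SwitchToPrevCharacter possesses PrevCharacter without updating either reference, printing an error if it is invalid.
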(event Custom|SwitchToNextCharacter
  (params (NewCharacter :type M%20Character%20Object%20Reference))
  (Utilities|IsValid NewCharacter
    (:Is%20Valid
      (Variables|Default|SetPrevCharacter (Variables|Default|GetCurrentCharacter))
      (Variables|Default|SetCurrentCharacter NewCharacter)
      (Pawn|Possess (Variables|Default|GetPrevCharacter)))))

(event Custom|SwitchToPrevCharacter
  (bind _prevcharacter (Variables|Default|GetPrevCharacter))
  (Utilities|IsValid _prevcharacter
    (:Is%20Valid
      (Pawn|Possess _prevcharacter))
    (:Is%20Not%20Valid
      (Development|PrintString "Cannot switch to prev character: prev character is null"))))

(event EventBeginPlay
  (bind _asmcharacter (Utilities|Casting|CastToMCharacter (Game|GetPlayerCharacter 0)))
  (Variables|Default|SetCurrentCharacter _asmcharacter))

(event EventTick
  (params (DeltaSeconds :type Float%20%28single-precision%29)))

(fn ConstructionScript)