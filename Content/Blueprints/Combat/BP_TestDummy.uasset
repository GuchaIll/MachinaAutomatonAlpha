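; Combat test dummy character that takes damage, reacts to hits and can be held airborne by an attacker, with a health display widget.
; AnyDamage applies a SetByCaller Gameplay Effect, picks a hit montage from the nearest of four directional components, and launches the dummy away from the damage causer.
; Loose gameplay tags mark air attachment, during which Tick tracks the attacker's attachment point until detach or landing.
; Face-player and spacing logic is disconnected.
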(event OnComponentBeginOverlap(CapsuleComponent)
  (params (OverlappedComponent :type Primitive%20Component%20Object%20Reference) (OtherActor :type Actor%20Object%20Reference) (OtherComp :type Primitive%20Component%20Object%20Reference) (OtherBodyIndex :type Integer) (bFromSweep :type Boolean) (SweepResult :type Hit%20Result%20Structure%20%28by%20ref%29)))

(event OnComponentEndOverlap(CapsuleComponent)
  (params (OverlappedComponent :type Primitive%20Component%20Object%20Reference) (OtherActor :type Actor%20Object%20Reference) (OtherComp :type Primitive%20Component%20Object%20Reference) (OtherBodyIndex :type Integer)))

(event Custom|Event%20Simulated%20Collision
  (bind _returnvalue (Transformation|GetActorLocation))
  (bind _attackdistance (Variables|Default|GetAttackDistance))
  (if (Utilities|DoesObjectImplementInterface (stale OnComponentBeginOverlap(CapsuleComponent) OtherActor) "/Game/Blueprints/Combat/BPI_Combat.BPI_Combat_C")
    (if (< (Math|Vector|VectorLength (- (Transformation|GetActorLocation (stale OnComponentBeginOverlap(CapsuleComponent) OtherActor)) _returnvalue)) _attackdistance)
      (AI|AIMoveTo (AI|GetAIController self) (+ _returnvalue (* (* _attackdistance (Math|Vector|Normalize (- (Transformation|GetActorLocation (stale OnComponentBeginOverlap(CapsuleComponent) OtherActor)) _returnvalue))) -1.0)) 0 -1.0 "Default" "Default" true true))))

(event Custom|Face%20Player)

(event EventBeginPlay
  (Utilities|FlowControl|Delay 0.5)
  (bind _aswbp_enemy_health_display (Utilities|Casting|CastToWBP_EnemyHealthDisplay (UserInterface|GetUserWidgetObject (Variables|Default|GetHealth%20Display))))
  (Default|CallEnemyRefSetUp _aswbp_enemy_health_display self))

(event EventAttachTargetinAir
  (params (AttachedActor :type Actor%20Object%20Reference))
  (bind _onsuccess (CallFunction|HasTag "(TagName=\"Combat.Attached\")"))
  (if (not _onsuccess)
    (CallFunction|AddTag "(GameplayTags=((TagName=\"Combat.Airborne\")))")
    (CallFunction|AddTag "(GameplayTags=((TagName=\"Combat.Attached\")))")
    (bind _attachedlocation (Class|BPICombat|GetAttachmentPoint(Message) AttachedActor))
    (Variables|Default|SetAttachmentPoint _attachedlocation)))

(event Game|Damage|EventAnyDamage
  (params (Damage :type Float%20%28single-precision%29) (DamageType :type Damage%20Type%20Object%20Reference) (InstigatedBy :type Controller%20Object%20Reference) (DamageCauser :type Actor%20Object%20Reference))
  (bind _mesh (Variables|Character|GetMesh))
  ;[0.15 0.15 0.15 0.5] Event Take Damage
  (bind _returnvalue (Ability|GameplayEffect|AssignTagSetbyCallerMagnitude (GameplayEffects|MakeOutgoingSpec (Variables|Default|GetAbilitySystem) "/Game/Blueprints/Combat/GameplayEffect/GE_DamageTest.GE_DamageTest_C" 0.0 (GameplayEffects|MakeEffectContext (Variables|Default|GetAbilitySystem))) "(TagName=\"Data.Damage\")" (* Damage -1.0)))
  (GameplayEffects|ApplyGameplayEffectSpecToSelf (Variables|Default|GetAbilitySystem) _returnvalue)
  (bind _hitdirection (CallFunction|CalculateHitDirection (Transformation|GetActorLocation DamageCauser)))
  (switch Utilities|FlowControl|Switch|SwitchonE_CombatDirection _hitdirection
    (:NewEnumerator0
      (Animation|Montage|PlayMontage _mesh "/Game/Animations/Ghost/Hit/MM_Lucy_Hit_F_Inplace_Montage.MM_Lucy_Hit_F_Inplace_Montage"
        (:then
          _)))
    (:NewEnumerator1
      (Animation|Montage|PlayMontage _mesh "/Game/Animations/Ghost/Hit/MM_Lucy_Hit_B_Inplace_Montage.MM_Lucy_Hit_B_Inplace_Montage"
        (:then
          _)))
    (:NewEnumerator2
      (Animation|Montage|PlayMontage _mesh "/Game/Animations/Ghost/Hit/MM_Lucy_Hit_L_Inplace_Montage.MM_Lucy_Hit_L_Inplace_Montage"
        (:then
          _)))
    (:NewEnumerator3
      (Animation|Montage|PlayMontage _mesh "/Game/Animations/Ghost/Hit/MM_Lucy_Hit_R_Inplace_Montage.MM_Lucy_Hit_R_Inplace_Montage"
        (:then
          _))))
  (Character|LaunchCharacter (* (* (Math|Vector|Normalize (- (Transformation|GetActorLocation DamageCauser) (Transformation|GetActorLocation))) (Variables|Default|GetKnockback%20Amt)) -1.0) true false))

(event EventUnattachTargetinAir
  (CallFunction|RemoveTag "(GameplayTags=((TagName=\"Combat.Airborne\")))")
  (CallFunction|RemoveTag "(GameplayTags=((TagName=\"Combat.Attached\")))"))

(event EventAddTag
  (params (AddTag :type Gameplay%20Tag%20Container%20Structure))
  (Ability|GameplayEffect|AddLooseGameplayTags self AddTag))

(event EventTick
  (params (DeltaSeconds :type Float%20%28single-precision%29))
  (bind _attachmentpoint (Variables|Default|GetAttachmentPoint))
  (bind _onsuccess (CallFunction|HasTag "(TagName=\"Combat.Attached\")"))
  (if _onsuccess
    (Utilities|IsValid _attachmentpoint
      (:Is%20Valid
        (Transformation|SetActorLocation (Math|Interpolation|VInterpTo (Transformation|GetWorldLocation _attachmentpoint) (Transformation|GetActorLocation) DeltaSeconds 1e+01) false false)))))

(event EventOnLanded
  (params (Hit :type Hit%20Result%20Structure%20%28by%20ref%29))
  (CallFunction|UnattachTargetinAir))

(fn ConstructionScript)

(fn CalculateHitDirection
  (params (HitLocationVector :type Vector))
  (bind _left (Variables|Default|Getleft))
  (bind _right (Variables|Default|Getright))
  (bind _back (Variables|Default|Getback))
  (bind _returnvalue (Transformation|GetWorldLocation _right))
  (bind _returnvalue_2 (Transformation|GetWorldLocation _left))
  (bind _returnvalue_3 (Transformation|GetWorldLocation _back))
  (bind _returnvalue_4 (Math|Vector|Distance2D(Vector) HitLocationVector _returnvalue_3))
  (bind _returnvalue_5 (Math|Vector|Distance2D(Vector) HitLocationVector _returnvalue_2))
  (bind _returnvalue_6 (Math|Vector|Distance2D(Vector) HitLocationVector _returnvalue))
  (LocalVariables|SetClosestHitDistance (Math|Vector|Distance2D(Vector) HitLocationVector (Transformation|GetWorldLocation (Variables|Default|Getfront))))
  (LocalVariables|SetClosestHitDirection "NewEnumerator0")
  (if (< _returnvalue_5 (LocalVariables|GetClosestHitDistance))
    (LocalVariables|SetClosestHitDistance _returnvalue_5)
    (LocalVariables|SetClosestHitDirection "NewEnumerator2"))
  (if (< _returnvalue_6 (LocalVariables|GetClosestHitDistance))
    (LocalVariables|SetClosestHitDistance _returnvalue_6)
    (LocalVariables|SetClosestHitDirection "NewEnumerator3"))
  (if (< _returnvalue_4 (LocalVariables|GetClosestHitDistance))
    (LocalVariables|SetClosestHitDistance _returnvalue_4)
    (LocalVariables|SetClosestHitDirection "NewEnumerator1"))
  (return (LocalVariables|GetClosestHitDirection) (LocalVariables|GetClosestHitDistance)))

(fn ActivateAbilitybyTag
  (params (GameplayTag :type Gameplay%20Tag%20Container%20Structure))
  (return false))

(fn GetAllTags
  (return ""))

(fn GetAttachmentPoint)

(fn GetAttackTarget
  (return 0))

(fn GetCombatState
  (return ""))

(fn HasTag
  (params (Tag :type Gameplay%20Tag%20Structure))
  (return (GameplayTags|HasMatchingGameplayTag (Ability|GetAbilitySystemComponent 0) Tag)))

(fn RemoveTag
  (params (GameplayTag :type Gameplay%20Tag%20Container%20Structure))
  (bind _returnvalue (Ability|GameplayEffect|RemoveLooseGameplayTags self GameplayTag))
  (return _returnvalue))

(fn TraceTarget
  (return false 0))