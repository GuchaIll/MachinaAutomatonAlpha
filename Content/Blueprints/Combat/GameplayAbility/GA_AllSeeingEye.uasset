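; All Seeing Eye gameplay ability that temporarily reveals enemy info displays on the avatar's potential targets.
; On activation it loops over the TargetSystem component's PotentialTargets and unhides EnemyInfoDisplay on each BP_EnemyBase, ending immediately without that component.
; A 15-second timer then ends the ability, hiding only the display of the last cast enemy rather than every revealed one.
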(event Custom|RemoveInfoWidget
  (Utilities|Time|ClearandInvalidateTimerbyHandle (stale Ability|EventActivateAbility _returnvalue_3))
  (Development|SetHiddeninGame (Variables|/Game/Blueprints/Enemy/BP_EnemyBase.BP_EnemyBase_C|GetEnemyInfoDisplay (stale Ability|EventActivateAbility _asbp_enemy_base)) true false)
  (Ability|EndAbility))

(event Ability|EventActivateAbility
  (bind _returnvalue (Ability|GetAvatarActorfromActorInfo))
  (bind _returnvalue_2 (Actor|GetComponentbyClass _returnvalue "/Script/GASPALS.TargetSystem"))
  (Utilities|IsValid _returnvalue_2
    (:Is%20Valid
      (for _array_element (Variables|/Script/GASPALS.TargetSystem|GetPotentialTargets _returnvalue_2)
        (bind _asbp_enemy_base (Utilities|Casting|CastToBP_EnemyBase _array_element))
        (Development|SetHiddeninGame (Variables|/Game/Blueprints/Enemy/BP_EnemyBase.BP_EnemyBase_C|GetEnemyInfoDisplay _asbp_enemy_base) false true))
      (bind _returnvalue_3 (Utilities|Time|SetTimerbyEvent (delegate Custom|RemoveInfoWidget) 15.0)))
    (:Is%20Not%20Valid
      (Ability|EndAbility))))

(event Ability|EventOnEndAbility
  (params (bWasCancelled :type Boolean)))