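; GA_Combo is the gameplay ability that executes one combo attack step when the next attack is ready.
; It turns buffered input into a next-move query, adding air velocity or an Ultimate launch as needed.
; On the EnterCombo tag, it checks spawned trigger-condition actors, orients and motion-warps toward the target, then plays the state's montage and applies its effects.
; Heavy attacks charge until tag removal or timeout; "D"-prefixed states jump to a Continue section.
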(event Custom|ForceChargeAttackRlease
  (Utilities|Time|ClearandInvalidateTimerbyHandle (stale Ability|EventActivateAbility _returnvalue_17))
  (|PlayMontageandWaitProxy "None" (.ActiveMontage (Utilities|Struct|BreakCombatState (stale Ability|EventActivateAbility _combatstate))) 1.0 "Release" false 1.0 0.0 false
    (:then
      (Class|BPICombat|RemoveTag(Message) (Ability|GetAvatarActorfromActorInfo) "(GameplayTags=((TagName=\"Combat.Charging\")))"))
    (:OnCompleted
      _)
    (:OnBlendOut
      _)
    (:OnInterrupted
      _)
    (:OnCancelled
      _))
  (Ability|EndAbility))

(event Custom|KeyReleased
  (params (TouchedActor :type Actor%20Object%20Reference) (ButtonReleased :type Key%20Structure :default "None"))
  (Development|PrintText (Class|KismetInputLibrary|KeyGetDisplayName ButtonReleased true)))

(event Ability|EventActivateAbility
  (bind _returnvalue (Ability|GetAvatarActorfromActorInfo))
  (bind _returnvalue_2 (Ability|GetAvatarActorfromActorInfo))
  (bind _returnvalue_3 (Ability|GetAvatarActorfromActorInfo))
  (bind _returnvalue_4 (Ability|GetAvatarActorfromActorInfo))
  (bind _returnvalue_5 (Ability|GetAvatarActorfromActorInfo))
  (bind _returnvalue_6 (Ability|GetAvatarActorfromActorInfo))
  (bind _returnvalue_7 (Ability|GetAvatarActorfromActorInfo))
  (bind _returnvalue_8 (Ability|GetAvatarActorfromActorInfo))
  (bind _returnvalue_9 (Ability|GetAvatarActorfromActorInfo))
  (bind _airattacktraveldistance (Variables|Default|GetAirAttackTravelDistance))
  (bind _returnvalue_10 (Actor|GetComponentbyClass _returnvalue_9 "/Script/MotionWarping.MotionWarpingComponent"))
  (bind _returnvalue_11 (Actor|GetComponentbyClass _returnvalue_8 "/Script/GASPALS.InputSubSystem"))
  (bind _returnvalue_12 (Transformation|GetActorForwardVector _returnvalue_6))
  (bind _returnvalue_13 (* _returnvalue_12 _airattacktraveldistance))
  (bind _onsuccess (Class|BPICombat|HasTag(Message) _returnvalue_8 "(TagName=\"Combat.NextAttackReady\")"))
  (if _onsuccess
    (Ability|CommitAbility)
    (Utilities|IsValid _returnvalue_11
      (:Is%20Valid
        (bind _returnvalue_14 (Class|InputSubSystem|ProcessInputBuffer _returnvalue_11))
        (Variables|Default|SetNewInput _returnvalue_14)
        (if (Utilities|Enum|Equal(Enum) _returnvalue_14 "Ultimate")
          (bind _onsuccess_2 (Class|BPICombat|HasTag(Message) _returnvalue_6 "(TagName=\"Combat.Airborne\")"))
          (if _onsuccess_2
            (Ability|EndAbility)
            (else
              (bind _lockedontarget (Class|BPICombat|GetAttackTarget(Message) _returnvalue_6))
              (Class|BPICombat|LaunchinAir(Message) _returnvalue_6 _lockedontarget)
              (Utilities|IsValid _lockedontarget
                (:Is%20Valid
                  (Class|BPICombat|AttachTargetinAir(Message) _lockedontarget _returnvalue_6)
                  (Class|BPICombat|QueryNextMove(Message) _returnvalue_5 _returnvalue_14 :!label _label))
                (:Is%20Not%20Valid
                  _))
              (Ability|Tasks|WaitGameplayTagAddToActor _returnvalue_5 "(TagName=\"Combat.EnterCombo\")" true
                (:Added
                  (bind _combatstate (Class|BPICombat|GetCombatState(Message) _returnvalue_5))
                  (Class|BPICombat|RemoveTag(Message) _returnvalue_5 "(GameplayTags=((TagName=\"Combat.EnterCombo\")))")
                  (bind _array_element (Utilities|Array|ForEachLoopwithBreak (.TriggerConditions (Utilities|Struct|BreakCombatState _combatstate)))
                    (:LoopBody
                      (bind _returnvalue_15 (Game|SpawnActorfromClass _array_element (Transformation|GetActorTransform _returnvalue_5) "Undefined" "MultiplyWithRoot" 0 _returnvalue_5 0))
                      (bind _returnvalue_16 (Class|CombatTriggerCondition|EvaluateTriggerCondition _returnvalue_15))
                      (if (not _returnvalue_16)
                        (Variables|Default|SetTriggerConditionMet false)))
                    (:Completed
                      (Development|PrintString (Utilities|GetDisplayName (.ActiveMontage (Utilities|Struct|BreakCombatState _combatstate))))
                      (if (Utilities|Enum|Equal(Enum) (Variables|Default|GetNewInput) "Jump")
                        (Ability|EndAbility)
                        (elif (Variables|Default|GetTriggerConditionMet)
                          (Class|MotionWarpingComponent|RemoveWarpTarget _returnvalue_10 "LockonTarget")
                          (bind _lockedontarget_2 (Class|BPICombat|GetAttackTarget(Message) _returnvalue_9))
                          (Development|PrintString (Utilities|GetDisplayName _lockedontarget_2) true true "(R=1.000000,G=0.000000,B=0.128734,A=1.000000)")
                          (Utilities|IsValid _lockedontarget_2
                            (:Is%20Valid
                              (Class|BPICombat|OrientAttacktoTarget(Message) _returnvalue 0 true)
                              (if (Utilities|String|StartsWith (Utilities|String|ToString(Name) (.StateName (Utilities|Struct|BreakCombatState _combatstate))) "D")
                                (Class|MotionWarpingComponent|AddorUpdateWarpTarget _returnvalue_10 (Utilities|Struct|MakeMotionWarpingTarget "LockonTarget" (+ (* (Math|Vector|Normalize (Math|Vector|RotateVector (Transformation|GetActorForwardVector _returnvalue_3) (Math|Rotator|FindLookatRotation (Transformation|GetActorLocation _lockedontarget_2) (Transformation|GetActorLocation _returnvalue_3)))) (Variables|Default|GetTarget%20Offset)) (Transformation|GetActorLocation _lockedontarget_2))) :!label _label_2)
                                (else
                                  (bind _inrange (CallFunction|CheckinRange _lockedontarget_2))
                                  (if _inrange
                                    (goto _label_2)
                                    (else
                                      _)))))
                            (:Is%20Not%20Valid
                              (Class|BPICombat|OrientAttacktoMovemet(Message) _returnvalue true)))
                          (|PlayMontageandWaitProxy "None" (.ActiveMontage (Utilities|Struct|BreakCombatState _combatstate)) (Variables|/Script/Engine.Actor|GetCustomTimeDilation (Ability|GetAvatarActorfromActorInfo)) "None" false 1.0 0.0 false
                            (:then
                              (Class|BPICombat|RemoveTag(Message) _returnvalue_7 "(GameplayTags=((TagName=\"Combat.ResetCombo\")))")
                              (Class|BPICombat|RemoveTag(Message) _returnvalue_7 "(GameplayTags=((TagName=\"Combat.NextAttackReady\")))")
                              (for _array_element_2 (.GameplayEffects (Utilities|Struct|BreakCombatState _combatstate))
                                (Ability|ApplyGameplayEffectToOwner _array_element_2))
                              (if (Utilities|Enum|Equal(Enum) (Variables|Default|GetNewInput) "HeavyAttack")
                                (Class|BPICombat|AddTag(Message) _returnvalue_2 "(GameplayTags=((TagName=\"Combat.Charging\")))")
                                (Ability|Tasks|WaitGameplayTagRemoveFromActor _returnvalue_2 "(TagName=\"Combat.Charging\")" true
                                  (:then
                                    (Development|PrintString "Tagwait")
                                    (bind _returnvalue_17 (Utilities|Time|SetTimerbyEvent (delegate Custom|ForceChargeAttackRlease) (Variables|Default|GetMaxChargeTime))))
                                  (:Removed
                                    (Utilities|Time|ClearandInvalidateTimerbyHandle _returnvalue_17)
                                    (|PlayMontageandWaitProxy "None" (.ActiveMontage (Utilities|Struct|BreakCombatState _combatstate)) 1.0 "Release" false 1.0 0.0 false
                                      (:then
                                        (Class|BPICombat|RemoveTag(Message) _returnvalue_2 "(GameplayTags=((TagName=\"Combat.Charging\")))"))
                                      (:OnCompleted
                                        _)
                                      (:OnBlendOut
                                        _)
                                      (:OnInterrupted
                                        _)
                                      (:OnCancelled
                                        _))
                                    (Ability|EndAbility)))
                                (elif (Utilities|String|StartsWith (Utilities|String|ToString(Name) (.StateName (Utilities|Struct|BreakCombatState _combatstate))) "D")
                                  (Utilities|FlowControl|Delay 0.2)
                                  (|PlayMontageandWaitProxy "" (.ActiveMontage (Utilities|Struct|BreakCombatState _combatstate)) 1.0 "Continue" false 1.0 0.0 false
                                    (:OnCompleted
                                      _)
                                    (:OnBlendOut
                                      _)
                                    (:OnInterrupted
                                      _)
                                    (:OnCancelled
                                      _))
                                  (Ability|EndAbility)
                                  (else
                                    (Ability|EndAbility)))))
                            (:OnCompleted
                              (Ability|EndAbility :!label _label_3))
                            (:OnBlendOut
                              (goto _label_3))
                            (:OnInterrupted
                              (goto _label_3))
                            (:OnCancelled
                              (goto _label_3)))
                          (else
                            (Ability|EndAbility))))))))))
          (else
            (bind _onsuccess_3 (Class|BPICombat|HasTag(Message) _returnvalue_4 "(TagName=\"Combat.Airborne\")"))
            (if _onsuccess_3
              (Development|PrintString (Utilities|String|ToString(Vector) (Math|Vector|MakeVector (.x _returnvalue_13) (.y _returnvalue_13) (.z _returnvalue_13))) true true "(R=1.000000,G=0.266065,B=0.000000,A=1.000000)")
              (Class|BPICombat|ApplyAirVelocity(Message) _returnvalue_4 (Math|Vector|MakeVector (.x _returnvalue_13) (.y _returnvalue_13) 5e+02))
              (goto _label)
              (else
                (goto _label))))))
      (:Is%20Not%20Valid
        (Ability|EndAbility)))
    (else
      (Ability|EndAbility))))

(event Ability|EventOnEndAbility
  (params (bWasCancelled :type Boolean)))

(fn CheckinRange
  (params (lockOnTarget :type Actor%20Object%20Reference))
  (if (<= (Transformation|GetDistanceTo lockOnTarget (Ability|GetAvatarActorfromActorInfo)) (Variables|Default|GetcomboMinDistance))
    (return true)
    (else
      (return false))))