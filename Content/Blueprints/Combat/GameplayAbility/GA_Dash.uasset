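; Dash gameplay ability that plays a directional slide dodge when the avatar has the Combat.NextAttackReady tag message.
; It swaps that tag for Combat.Dash, snaps the character to control yaw, then disables automatic movement rotation a tick later.
; Movement input selects one of four root-motion montages, defaulting to backward.
; The ability ends right after starting the montage, removing Combat.Dash while the montage plays on.
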(event Ability|EventActivateAbility
  (bind _returnvalue (Ability|GetAvatarActorfromActorInfo))
  (bind _onsuccess (Class|BPICombat|HasTag(Message) _returnvalue "(TagName=\"Combat.NextAttackReady\")"))
  (if _onsuccess
    (bind _ascbp_sandbox_character (Utilities|Casting|CastToCBP_SandboxCharacter _returnvalue))
    (Class|BPICombat|RemoveTag(Message) _ascbp_sandbox_character "(GameplayTags=((TagName=\"Combat.NextAttackReady\")))")
    (Class|BPICombat|AddTag(Message) _ascbp_sandbox_character "(GameplayTags=((TagName=\"Combat.Dash\")))")
    (Transformation|SetActorRotation _ascbp_sandbox_character (Math|Rotator|MakeRotator 0.0 0.0 (.yaw (Pawn|GetControlRotation _ascbp_sandbox_character :!class /Script/Engine.Pawn))))
    (Utilities|FlowControl|DelayUntilNextTick)
    (Variables|/Script/Engine.CharacterMovementComponent|SetbUseControllerDesiredRotation (Variables|/Script/Engine.Character|GetCharacterMovement _ascbp_sandbox_character) false)
    (Variables|/Script/Engine.CharacterMovementComponent|SetbOrientRotationToMovement (Variables|/Script/Engine.Character|GetCharacterMovement _ascbp_sandbox_character) false)
    (if (> (Math|Vector|VectorLength (Variables|/Script/Engine.MovementComponent|GetVelocity (Variables|/Script/Engine.Character|GetCharacterMovement _ascbp_sandbox_character))) 1.0)
      (if (> (.Y (Math|Vector2D|BreakVector2D (Variables|/Game/Blueprints/CBP_SandboxCharacter.CBP_SandboxCharacter_C|GetMovementInput _ascbp_sandbox_character))) 0.05)
        (Variables|Default|SetDirection "NewEnumerator0")
        (elif (< (.Y (Math|Vector2D|BreakVector2D (Variables|/Game/Blueprints/CBP_SandboxCharacter.CBP_SandboxCharacter_C|GetMovementInput _ascbp_sandbox_character))) -0.05)
          (Variables|Default|SetDirection "NewEnumerator1" :!label _label)
          (elif (> (.X (Math|Vector2D|BreakVector2D (Variables|/Game/Blueprints/CBP_SandboxCharacter.CBP_SandboxCharacter_C|GetMovementInput _ascbp_sandbox_character))) 0.05)
            (Variables|Default|SetDirection "NewEnumerator3")
            (elif (< (.X (Math|Vector2D|BreakVector2D (Variables|/Game/Blueprints/CBP_SandboxCharacter.CBP_SandboxCharacter_C|GetMovementInput _ascbp_sandbox_character))) -0.05)
              (Variables|Default|SetDirection "NewEnumerator2")
              (else
                (goto _label))))))
      (else
        (goto _label)))
    (Utilities|Dodge)
    (Ability|EndAbility)
    (else
      (Ability|EndAbility))))

(event Ability|EventOnEndAbility
  (params (bWasCancelled :type Boolean))
  (Class|BPICombat|RemoveTag(Message) (Ability|GetAvatarActorfromActorInfo) "(GameplayTags=((TagName=\"Combat.Dash\")))"))