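; Gameplay ability that throws a projectile from the player camera and follows a hit with a dash punch.
; Activation plays a taunt montage, spawns BP_Projectile along the camera's forward vector, and binds its overlap event alongside a miss timeout.
; On overlap, the avatar orients to the target and, if within MaxEngageDistance, motion-warps to an offset point during the punch montage.
; The ability ends as that montage starts, or on a miss or out-of-range hit.
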(event Custom|EngageCombat
  (params (AttackedTarget :type Actor%20Object%20Reference) (HitResult :type Hit%20Result%20Structure))
  (bind _returnvalue (Transformation|GetActorLocation AttackedTarget))
  (bind _returnvalue_2 (Ability|GetAvatarActorfromActorInfo))
  (bind _returnvalue_3 (Actor|GetComponentbyClass _returnvalue_2 "/Script/MotionWarping.MotionWarpingComponent"))
  (Utilities|Time|ClearandInvalidateTimerbyHandle (stale Ability|EventActivateAbility _returnvalue_4))
  (Utilities|IsValid AttackedTarget
    (:Is%20Valid
      (Class|MotionWarpingComponent|RemoveWarpTarget _returnvalue_3 "LockonTarget")
      (Development|PrintString (Utilities|GetDisplayName 0) true true "(R=1.000000,G=0.000000,B=0.128734,A=1.000000)")
      (Utilities|IsValid AttackedTarget
        (:Is%20Valid
          (Class|BPICombat|OrientAttacktoTarget(Message) (Ability|GetAvatarActorfromActorInfo) AttackedTarget true)
          (bind _inrange (CallFunction|CheckinRange AttackedTarget))
          (if _inrange
            (Class|MotionWarpingComponent|AddorUpdateWarpTarget _returnvalue_3 (Utilities|Struct|MakeMotionWarpingTarget "LockonTarget" (+ (* (Math|Vector|Normalize (Math|Vector|RotateVector (Transformation|GetActorForwardVector _returnvalue_2) (Math|Rotator|FindLookatRotation _returnvalue (Transformation|GetActorLocation _returnvalue_2)))) (Variables|Default|GetTargetOffset)) _returnvalue)))
            (|PlayMontageandWaitProxy "None" "/Game/Animations/Ghost/Combat/Fighter_DashPunch_Montage.Fighter_DashPunch_Montage" (Variables|/Script/Engine.Actor|GetCustomTimeDilation (Ability|GetAvatarActorfromActorInfo)) "None" false 1.0 0.0 false
              (:then
                _)
              (:OnCompleted
                _)
              (:OnBlendOut
                _)
              (:OnInterrupted
                _))
            (Ability|EndAbility)
            (else
              (Ability|EndAbility))))
        (:Is%20Not%20Valid
          (Ability|EndAbility))))
    (:Is%20Not%20Valid
      (Ability|EndAbility))))

(event Custom|Projectile%20Miss
  (Utilities|Time|ClearandInvalidateTimerbyHandle (stale Ability|EventActivateAbility _returnvalue_4))
  (EventDispatchers|UnbindEventfromOnTargetBeganOverlap (stale Ability|EventActivateAbility _returnvalue_3) (delegate Custom|EngageCombat))
  (Ability|EndAbility))

(event Ability|EventActivateAbility
  (bind _returnvalue (Game|GetPlayerCameraManager 0))
  (bind _returnvalue_2 (Transformation|GetActorTransform _returnvalue))
  (|PlayMontageandWaitProxy "None" "/Game/Animations/Ghost/Combat/Fighter_Taunt_Montage.Fighter_Taunt_Montage" (Variables|/Script/Engine.Actor|GetCustomTimeDilation (Ability|GetAvatarActorfromActorInfo)) "None" false 1.0 0.0 false
    (:then
      (bind _returnvalue_3 (Game|SpawnActorfromClass "/Game/Blueprints/Combat/Projectile/BP_Projectile.BP_Projectile_C" (Math|Transform|MakeTransform (+ (.location _returnvalue_2) (* (Transformation|GetActorForwardVector _returnvalue) 2e+02)) (.rotation _returnvalue_2)) "Undefined" "MultiplyWithRoot" 0 0))
      (EventDispatchers|BindEventtoOnTargetBeganOverlap _returnvalue_3 (delegate Custom|EngageCombat))
      (bind _returnvalue_4 (Utilities|Time|SetTimerbyEvent (delegate Custom|Projectile%20Miss) 8.0)))))

(event Ability|EventOnEndAbility
  (params (bWasCancelled :type Boolean)))

(fn CheckinRange
  (params (lockOnTarget :type Actor%20Object%20Reference))
  (if (<= (Transformation|GetDistanceTo lockOnTarget (Ability|GetAvatarActorfromActorInfo)) (Variables|Default|GetMaxEngageDistance))
    (return true)
    (else
      (return false))))