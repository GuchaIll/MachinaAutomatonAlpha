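; Gameplay ability that applies a temporary time dilation, setting separate rates for the world and for the avatar.
; Activation sets global and avatar dilation, then for a CBP_SandboxCharacter scales mesh animation rate, raises walk speed and starts a Duration timer.
; The timer event resets these to hardcoded defaults and ends the ability.
; A failed cast ends the ability immediately without restoring either dilation.
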(event Custom|EndTimeDilation
  (Utilities|Time|SetGlobalTimeDilation 1.0)
  (Variables|/Script/Engine.Actor|SetCustomTimeDilation (Ability|GetAvatarActorfromActorInfo) 1.0)
  (Variables|/Script/Engine.SkeletalMeshComponent|SetGlobalAnimRateScale (Variables|/Script/Engine.Character|GetMesh (stale Ability|EventActivateAbility _ascbp_sandbox_character)) 1.0)
  (Variables|/Script/Engine.CharacterMovementComponent|SetMaxWalkSpeed (Variables|/Script/Engine.Character|GetCharacterMovement (stale Ability|EventActivateAbility _ascbp_sandbox_character)) 5e+02)
  (Ability|EndAbility))

(event Ability|EventActivateAbility
  (bind _returnvalue (Ability|GetAvatarActorfromActorInfo))
  (Utilities|Time|SetGlobalTimeDilation (Variables|Default|GetGlobalTimeDilationRate))
  (Variables|/Script/Engine.Actor|SetCustomTimeDilation _returnvalue (Variables|Default|GetPlayerTimeDilationRate))
  (bind _ascbp_sandbox_character (Utilities|Casting|CastToCBP_SandboxCharacter _returnvalue)
    (:then
      (Variables|/Script/Engine.SkeletalMeshComponent|SetGlobalAnimRateScale (Variables|/Script/Engine.Character|GetMesh _ascbp_sandbox_character) (Variables|Default|GetPlayerTimeDilationRate))
      (Variables|/Script/Engine.CharacterMovementComponent|SetMaxWalkSpeed (Variables|/Script/Engine.Character|GetCharacterMovement _ascbp_sandbox_character) 1e+03)
      (Utilities|Time|SetTimerbyEvent (delegate Custom|EndTimeDilation) (Variables|Default|GetDuration)))
    (:CastFailed
      (Ability|EndAbility))))

(event Ability|EventOnEndAbility
  (params (bWasCancelled :type Boolean)))