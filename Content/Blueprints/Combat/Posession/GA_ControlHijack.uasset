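; Gameplay ability that lets the player temporarily take control of a selected target.
; A target selection widget supplies the target, which gets hidden with collision and tick disabled while PC_Sandbox switches control to a substitute character.
; A duration timer or that character's switch-back event restores the previous character and target, destroys the substitute and ends the ability.
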(event Custom|SetNewControlTarget
  (params (HijackedTarget :type M%20Character%20Object%20Reference))
  (Utilities|IsValid HijackedTarget
    (:Is%20Valid
      (Rendering|SetActorHiddenInGame HijackedTarget true)
      (Collision|SetActorEnableCollision HijackedTarget false)
      (Actor|Tick|SetActorTickEnabled HijackedTarget)
      (bind _aspc_sandbox (Utilities|Casting|CastToPC_Sandbox (Game|GetPlayerController 0))
        (:then
          (bind _controlledpawn (Default|SwitchtoNextCharacter _aspc_sandbox HijackedTarget))
          (Utilities|IsValid _controlledpawn
            (:Is%20Valid
              (EventDispatchers|BindEventtoSwitchBacktoOwner _controlledpawn (delegate Custom|OnEarlyReturnToOwner))
              (bind _returnvalue (Utilities|Time|SetTimerbyEvent (delegate Custom|ResetControllerToOwner) (Variables|Default|GetControlledDuration))))
            (:Is%20Not%20Valid
              (Ability|EndAbility))))
        (:CastFailed
          (Ability|EndAbility))))
    (:Is%20Not%20Valid
      (Ability|EndAbility))))

(event Custom|ResetControllerToOwner
  (Utilities|Time|ClearandInvalidateTimerbyHandle (stale Custom|SetNewControlTarget _returnvalue))
  (bind _aspc_sandbox (Utilities|Casting|CastToPC_Sandbox (Game|GetPlayerController 0)))
  (Default|SwitchtoPrevCharacter (stale Custom|SetNewControlTarget _aspc_sandbox))
  (Rendering|SetActorHiddenInGame (stale Custom|SetNewControlTarget HijackedTarget) false)
  (Collision|SetActorEnableCollision (stale Custom|SetNewControlTarget HijackedTarget) true)
  (Actor|Tick|SetActorTickEnabled (stale Custom|SetNewControlTarget HijackedTarget) true)
  (Actor|DestroyActor (stale Custom|SetNewControlTarget _controlledpawn))
  (Ability|EndAbility))

(event Custom|OnEarlyReturnToOwner
  (Utilities|Time|ClearandInvalidateTimerbyHandle (stale Custom|SetNewControlTarget _returnvalue))
  (bind _aspc_sandbox (Utilities|Casting|CastToPC_Sandbox (Game|GetPlayerController 0)))
  (Default|SwitchtoPrevCharacter (stale Custom|SetNewControlTarget _aspc_sandbox))
  (Rendering|SetActorHiddenInGame (stale Custom|SetNewControlTarget HijackedTarget) false)
  (Collision|SetActorEnableCollision (stale Custom|SetNewControlTarget HijackedTarget) true)
  (Actor|Tick|SetActorTickEnabled (stale Custom|SetNewControlTarget HijackedTarget) true)
  (Actor|DestroyActor (stale Custom|SetNewControlTarget _controlledpawn))
  (Ability|EndAbility))

(event Ability|EventActivateAbility
  (bind _returnvalue (UserInterface|CreateWidget "/Game/Blueprints/Combat/Posession/WBP_ControlHijackTargetSelect.WBP_ControlHijackTargetSelect_C" (Game|GetPlayerController 0)))
  (UserInterface|Viewport|AddtoViewport _returnvalue 0)
  (EventDispatchers|BindEventtoHijackTargetSelected _returnvalue (delegate Custom|SetNewControlTarget)))

(event Ability|EventOnEndAbility
  (params (bWasCancelled :type Boolean)))