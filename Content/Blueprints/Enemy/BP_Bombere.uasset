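; BP_Bombere is an enemy Blueprint that gains an explosion attack through the Gameplay Ability System.
; On BeginPlay it runs the parent logic, then grants GA_Explosion to its Ability System Component; activation happens outside this graph.
; GetAttackTarget returns the locked-on target, while TraceTarget always reports no hit.
; Tick and overlap events are disabled.
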(event EventBeginPlay
  (|CallParentFunction)
  (GameplayAbilities|GiveAbility (Ability|GetAbilitySystemComponent 0) "/Game/Blueprints/Enemy/GameplayAbility/GA_Explosion.GA_Explosion_C" 0 -1))

(event Collision|EventActorBeginOverlap
  (params (OtherActor :type Actor%20Object%20Reference))
  (|CallParentFunction OtherActor) ; This node is disabled and will not be called.\nDrag off pins to build functionality.
)

(event EventTick
  (params (DeltaSeconds :type Float%20%28single-precision%29))
  (|CallParentFunction DeltaSeconds) ; This node is disabled and will not be called.\nDrag off pins to build functionality.
)

(fn ConstructionScript
  (|CallParentFunction))

(fn GetAttackTarget
  (return (Variables|Default|GetLockedOnTarget)))

(fn TraceTarget
  (return false 0))