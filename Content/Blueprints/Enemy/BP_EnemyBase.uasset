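; BP_EnemyBase is a base enemy Blueprint that uses the Gameplay Ability System and carries an info display widget.
; On BeginPlay it passes its class to the WBP_EnemyInfoDisplayPanel for setup, then initializes abilities, skipping both if the widget cast fails.
; InitializeAbility grants the ability from every EnemyData table row whose CharacterClass exactly matches the enemy's class.
; ActivateAbilityByTag wraps tag-based activation on the ability system and returns the result.
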(event EventBeginPlay
  (|CallParentFunction)
  (bind _aswbp_enemy_info_display_panel (Utilities|Casting|CastToWBP_EnemyInfoDisplayPanel (UserInterface|GetWidget (Variables|Default|GetEnemyInfoDisplay))))
  (Variables|/Game/Blueprints/Combat/Widgets/WBP_EnemyInfoDisplayPanel.WBP_EnemyInfoDisplayPanel_C|SetEnemyRef _aswbp_enemy_info_display_panel (Utilities|GetClass self))
  (Default|SetUpData _aswbp_enemy_info_display_panel)
  (CallFunction|InitializeAbility))

(event Collision|EventActorBeginOverlap
  (params (OtherActor :type Actor%20Object%20Reference)))

(event EventTick
  (params (DeltaSeconds :type Float%20%28single-precision%29))
  (|CallParentFunction DeltaSeconds) ; This node is disabled and will not be called.\nDrag off pins to build functionality.
)

(fn ConstructionScript
  (|CallParentFunction))

(fn ActivateAbilitybyTag
  (params (GameplayTag :type Gameplay%20Tag%20Container%20Structure))
  (bind _returnvalue (Abilities|TryActivateAbilitiesbyTag (Variables|Default|GetAbilitySystem) GameplayTag true))
  (return _returnvalue))

(fn InitializeAbility
  (bind _enemydata (Variables|Default|GetEnemyData))
  (bind _outrownames (DataTable|GetDataTableRowNames _enemydata))
  (bind _array_element (Utilities|Array|ForEachLoopwithBreak _outrownames)
    (:LoopBody
      (bind _returnvalue (Utilities|GetDataTableRow _enemydata _array_element)
        (:then
          (if (== (.CharacterClass (Utilities|Struct|BreakST_PossessionMap _returnvalue)) (Utilities|GetClass self))
            (GameplayAbilities|GiveAbility (Variables|Default|GetAbilitySystem) (.Ability (Utilities|Struct|BreakST_PossessionMap _returnvalue)) 0 -1)))))))