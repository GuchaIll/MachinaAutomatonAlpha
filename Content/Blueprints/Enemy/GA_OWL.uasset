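; GA_OWL is an enemy gameplay ability that performs an air-kick melee attack.
; On activation it starts the kick montage and immediately runs a sphere overlap for pawns around the avatar, without waiting for an anim notify.
; Each hit actor lacking the "Enemy" tag takes damage and triggers newly spawned camera shake and zoom-in actors.
; The ability ends when the montage completes, blends out, is interrupted or is cancelled.
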(event Ability|EventActivateAbility
  (bind _returnvalue (Ability|GetAvatarActorfromActorInfo))
  (|PlayMontageandWaitProxy "None" "/Game/Animations/Ghost/AirAttacks/MM_Lucy_Air_Kick_04_Root_Montage.MM_Lucy_Air_Kick_04_Root_Montage" 1.0 "None" true 1.0 0.0 false
    (:then
      (bind (_outactors _returnvalue_2) (Collision|SphereOverlapActors (Transformation|GetActorLocation _returnvalue) 1e+02 (Utilities|Array|MakeArray "ObjectTypeQuery3") 0 (Utilities|Array|MakeArray _returnvalue)))
      (if _returnvalue_2
        (for _array_element _outactors
          (if (not (Actor|ActorHasTag _array_element "Enemy"))
            (Game|Damage|ApplyDamage _array_element 1e+02 0 0)
            (bind _returnvalue_3 (Game|SpawnActorfromClass "/Game/Blueprints/Cameras/BP_CameraShake.BP_CameraShake_C" (Math|Transform|MakeTransform "0, 0, 0") "Undefined" "MultiplyWithRoot" 0 0))
            (Default|PlayAnimCam _returnvalue_3)
            (bind _returnvalue_4 (Game|SpawnActorfromClass "/Game/Blueprints/Cameras/BP_CameraZoomInActor.BP_CameraZoomInActor_C" (Math|Transform|MakeTransform "0, 0, 0") "Undefined" "MultiplyWithRoot" 0 0))
            (Default|PlayAnimCam _returnvalue_4)))))
    (:OnCompleted
      (Ability|EndAbility :!label _label))
    (:OnBlendOut
      (goto _label))
    (:OnInterrupted
      (goto _label))
    (:OnCancelled
      (goto _label))))

(event Ability|EventOnEndAbility
  (params (bWasCancelled :type Boolean)))