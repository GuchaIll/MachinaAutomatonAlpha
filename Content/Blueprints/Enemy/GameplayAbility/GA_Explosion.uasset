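; Enemy gameplay ability that sets off a delayed explosion at its avatar's location.
; Activation spawns a cloud particle effect and starts a timer for the blast, which plays a Niagara effect and sphere-traces for pawns with debug drawing on.
; Any hit triggers radial damage with falloff, using fixed radii independent of the trace's ExplosionAffectDistance.
; The ability ends after the blast whether or not anything was hit.
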(event Custom|Explosion
  (bind _returnvalue (Ability|GetAvatarActorfromActorInfo))
  (bind _returnvalue_2 (Transformation|GetActorLocation _returnvalue))
  (Niagara|SpawnSystematLocation "/Game/Assets/Niagara/NewNiagaraSystem.NewNiagaraSystem" _returnvalue_2)
  (bind _returnvalue_3 (Collision|MultiSphereTraceForObjects _returnvalue_2 _returnvalue_2 (Variables|Default|GetExplosionAffectDistance) (Utilities|Array|MakeArray "ObjectTypeQuery3") false 0 "ForDuration" false))
  (if _returnvalue_3
    (Class|GameplayStatics|ApplyRadialDamagewithFalloff 5e+02 2e+01 _returnvalue_2 1e+02 2e+02 0.2 0 0 _returnvalue 0 "ECC_Visibility")
    (Ability|EndAbility)
    (else
      (Ability|EndAbility))))

(event Ability|EventActivateAbility
  (Effects|SpawnEmitteratLocation "/Game/Polar/Particles/P_Clouds.P_Clouds" "0, 0, 0")
  (Utilities|Time|SetTimerbyEvent (delegate Custom|Explosion) (Variables|Default|GetExplosionTimeDelay)))

(event Ability|EventOnEndAbility
  (params (bWasCancelled :type Boolean)))