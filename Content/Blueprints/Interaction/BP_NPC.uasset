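; NPC Blueprint that opens a dialogue box when interacted with and tracks whether an interaction is active.
; TryInteractwith reuses an existing top-level WBP_DialogueBox and starts DialogueStates, or creates a new widget without starting DialogueStates here.
; Either path hands the widget a reference back to this NPC.
; EndInteraction clears the flag and stops DialogueStates, while GetNextResponse is an empty event.
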(event Custom|End%20Interaction
  (Variables|Default|SetisInteracting false)
  (Class|SMStateMachineComponent|Stop (Variables|Default|GetDialogueStates)))

(event EventBeginPlay)

(event Collision|EventActorBeginOverlap
  (params (OtherActor :type Actor%20Object%20Reference)))

(event EventTick
  (params (DeltaSeconds :type Float%20%28single-precision%29)))

(event EventTryInteractwith
  (if (not (Variables|Default|GetisInteracting))
    (Variables|Default|SetisInteracting true)
    (bind _foundwidgets (Widget|GetAllWidgetsOfClass "/Game/Blueprints/Interaction/WBP_DialogueBox.WBP_DialogueBox_C" true))
    (if (!= (Utilities|Array|Length _foundwidgets) 0)
      (bind _output_get (Variables|Default|SetDialogueWidget (Utilities|Array|Get(acopy) _foundwidgets)))
      (Variables|/Game/Blueprints/Interaction/WBP_DialogueBox.WBP_DialogueBox_C|SetNPCRef _output_get self)
      (Class|SMStateMachineComponent|Start (Variables|Default|GetDialogueStates))
      (else
        (bind _returnvalue (UserInterface|CreateWidget "/Game/Blueprints/Interaction/WBP_DialogueBox.WBP_DialogueBox_C" (Game|GetPlayerController 0) self))
        (bind _output_get_2 (Variables|Default|SetDialogueWidget _returnvalue))
        (UserInterface|Viewport|AddtoViewport _output_get_2 0)))))

(event EventGetNextResponse)

(fn ConstructionScript)